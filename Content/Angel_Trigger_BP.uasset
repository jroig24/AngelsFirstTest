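; Trigger actor that switches a set of assigned Angel actors to a configured state when the player enters it.
; Each overlap by player pawn 0 decrements MinOverlapCount, so activation can wait until a set number of entries.
; At zero or below, it writes AngelState to every valid entry in AngelsToActivate.
; The trigger destroys itself from inside that loop, so it persists if no entry is valid.
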(event `self.ReceiveActorBeginOverlap`
  (params (OtherActor :type "Actor Object Reference"))
  (if (== OtherActor (`GameplayStatics.GetPlayerPawn` 0))
    (bind _output_get (set `self.minOverlapCount` (- (`self.minOverlapCount`) 1)))
    (if (<= _output_get 0)
      (for _array_element (`self.AngelsToActivate`)
        (`/Engine/EditorBlueprintResources/StandardMacros.IsValid` _array_element
          (:`Is Valid`
            (set `/Game/ThirdPersonBP/Blueprints/Angel.state` (`self.angelState`) _array_element)
            (`self.K2_DestroyActor`)))))))

(fn `UserConstructionScript`)