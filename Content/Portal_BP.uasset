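; Portal actor that teleports the player pawn to a linked TargetPortal when the pawn overlaps it.
; The location math resolves to the target's exact position, and rotation is left unchanged.
; Before moving, it clears CanTeleport on the destination to prevent bouncing back, and end overlap re-arms it.
; That flag is cleared before the player check, so any overlapping actor disables the destination.
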(event `self.ReceiveActorEndOverlap`
  (params (OtherActor :type "Actor Object Reference"))
  (set `self.canTeleport` true))

(event `self.ReceiveBeginPlay`
  (set `self.canTeleport` true))

(event `self.ReceiveActorBeginOverlap`
  (params (OtherActor :type "Actor Object Reference"))
  (bind _returnvalue (`GameplayStatics.GetPlayerPawn` 0))
  (bind _targetportal (`self.TargetPortal`))
  (bind _returnvalue_2 (`self.K2_GetActorLocation` _returnvalue))
  (if (`self.canTeleport`)
    (`/Engine/EditorBlueprintResources/StandardMacros.IsValid` _targetportal
      (:`Is Valid`
        (bind _asportal_bp (cast `/Game/Portal_BP` _targetportal))
        (set `/Game/Portal_BP.canTeleport` false _asportal_bp)
        (if (== OtherActor _returnvalue)
          (`self.K2_SetActorLocation` _returnvalue (+ _returnvalue_2 (- (`self.K2_GetActorLocation` _targetportal) _returnvalue_2)) false true))))))

(fn `UserConstructionScript`)